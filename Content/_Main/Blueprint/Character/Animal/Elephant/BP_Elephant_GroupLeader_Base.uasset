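; Base Blueprint for an elephant group leader character that sets up its tusks according to the animal's age.
; The construction script gives adults a random skeletal mesh from the tusk array and snaps it to the tusk socket on the body mesh.
; For any other age status, it clears the tusk mesh.
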(fn `UserConstructionScript`
  (if (`|EnumEquality` (`self.GetAnimalAgeStatus`) "EAS_Adult")
    (`SkeletalMeshComponent.SetSkeletalMeshAsset` (`self.ElephantTusksMesh`) (`KismetArrayLibrary.Array_Random` (`self.Tusks Array`)))
    (`SceneComponent.K2_AttachToComponent` (`self.ElephantTusksMesh`) (`self.Mesh`) "TuskSocket" "SnapToTarget" "SnapToTarget" "SnapToTarget" true)
    (else
      (`SkeletalMeshComponent.SetSkeletalMeshAsset` (`self.ElephantTusksMesh`) null))))