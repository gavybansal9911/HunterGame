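; BP_Ranger is the Ranger character Blueprint, handling animal-interaction motion warping and debug hotkeys.
; SetWarpTarget casts the interaction target to BaseAnimal and feeds its head component transform to MotionWarping as the "AnimalInteraction" target.
; Number keys trigger test actions: a noise with explosion effects, AI damage events reported on the first enemy or lion found, and a printout of the content array.
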(event `Set Warp Target`
  (bind _returnvalue (`self.GetInteractionTargetActor`))
  (`/Engine/EditorBlueprintResources/StandardMacros.IsValid` _returnvalue
    (:`Is Valid`
      (bind _asbase_animal (cast `BaseAnimal` _returnvalue))
      (`MotionWarpingComponent.AddOrUpdateWarpTargetFromTransform` (`self.MotionWarping`) "AnimalInteraction" (`SceneComponent.K2_GetComponentToWorld` (`BaseAnimal.AnimalHead_SceneComponent` _asbase_animal))))))

(event `Key|One`
  (params (Key :type "Key Structure"))
  (bind _returnvalue (`self.K2_GetActorLocation`))
  (:`Pressed`
    (`self.MakeNoise` 1.0 null (`self.K2_GetActorLocation`))
    (`GameplayStatics.SpawnEmitterAtLocation` "/Game/StarterContent/Particles/P_Explosion.P_Explosion" _returnvalue)
    (`GameplayStatics.PlaySoundAtLocation` "/Game/StarterContent/Audio/Explosion01.Explosion01" _returnvalue (struct) 1.0 1.0 0.0 null null null null)))

(event `Key|Two`
  (params (Key :type "Key Structure"))
  (:`Pressed`
    (bind _returnvalue (`GameplayStatics.GetActorOfClass` "/Game/_Main/AI/EnemyAI/BP_EnemyBase.BP_EnemyBase_C"))
    (`AISense_Damage.ReportDamageEvent` _returnvalue self 10.0 (`self.K2_GetActorLocation`))))

(event `Key|Five`
  (params (Key :type "Key Structure"))
  (:`Pressed`
    (for (_array_element _array_index) (`self.GetContentArray`)
      (`KismetSystemLibrary.PrintString` (`KismetTextLibrary.Conv_TextToString` (`|FormatText` "{Index}: {Name} {Quantity}" _array_index (break `SlotData` _array_element) (`.Quantity` (break `SlotData` _array_element))))))))

(event `Key|Six`
  (params (Key :type "Key Structure"))
  (:`Pressed`
    (bind _returnvalue (`GameplayStatics.GetActorOfClass` "/Game/_Main/Blueprint/Character/Animal/Lion/BP_Lion_Base.BP_Lion_Base_C"))
    (`AISense_Damage.ReportDamageEvent` _returnvalue self 10.0 (`self.K2_GetActorLocation`))))

(fn `UserConstructionScript`)