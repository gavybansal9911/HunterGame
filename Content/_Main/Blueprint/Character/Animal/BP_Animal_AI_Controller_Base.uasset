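; Base AI controller for animal characters that runs behavior trees on request.
; RunBT starts the supplied tree asset, while StopBTExecution is an unimplemented stub that only prints a TODO message.
; Each tick, when the blackboard is valid, it draws a thick debug line from the controlled pawn to the PointOfInterest vector stored in the blackboard.
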(event `Run BT`
  (params (BTAsset :type "BehaviorTree Object Reference"))
  (`self.RunBehaviorTree` BTAsset))

(event `Stop BT Execution`
  (`KismetSystemLibrary.PrintString` "TODO: Implement Stop BT Execution function!"))

(event `self.ReceiveTick`
  (params (DeltaSeconds :type "Float (single-precision)"))
  (bind _returnvalue (`AIBlueprintHelperLibrary.GetBlackboard` null))
  (`/Engine/EditorBlueprintResources/StandardMacros.IsValid` _returnvalue
    (:`Is Valid`
      (`KismetSystemLibrary.DrawDebugLine` (`self.K2_GetActorLocation` (`self.K2_GetPawn`)) (`BlackboardComponent.GetValueAsVector` _returnvalue "PointOfInterest") (struct :`R` 1.0 :`G` 0.017847 :`A` 1.0) 0.0 10.0))))

(fn `UserConstructionScript`)